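; Floor actor that assembles four referenced room actors into one level of a stacked layout.
; The construction script sets the floor's height from FloorNumber at world X/Y zero, then attaches each room to it.
; Each room then gets a different quarter-turn rotation and a default zero location through a world-space set, so rooms do not inherit the floor's height.
; The event graph has no runtime logic.
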(event `self.ReceiveBeginPlay`)

(fn `UserConstructionScript`
  (bind _room0 (`self.Room0`))
  (bind _room1 (`self.Room1`))
  (bind _room2 (`self.Room2`))
  (bind _room3 (`self.Room3`))
  (`self.K2_SetActorLocation` (`KismetMathLibrary.MakeVector` 0.0 0.0 (* (`self.FloorNumber`) 10.0)))
  (`self.K2_AttachToActor` _room0 self "None" "KeepRelative" "KeepRelative" "KeepRelative" true)
  (`self.K2_SetActorLocationAndRotation` _room0 (0.0 0.0 0.0) (struct :`Yaw` 180.0) false false)
  (`self.K2_AttachToActor` _room1 self "None" "KeepRelative" "KeepRelative" "KeepRelative" true)
  (`self.K2_SetActorLocationAndRotation` _room1 (0.0 0.0 0.0) (struct :`Yaw` 90.0) false false)
  (`self.K2_AttachToActor` _room2 self "None" "KeepRelative" "KeepRelative" "KeepRelative" true)
  (`self.K2_SetActorLocationAndRotation` _room2 (0.0 0.0 0.0) (struct :`Yaw` 270.0) false false)
  (`self.K2_AttachToActor` _room3 self "None" "KeepRelative" "KeepRelative" "KeepRelative" true)
  (`self.K2_SetActorLocationAndRotation` :`self` _room3))
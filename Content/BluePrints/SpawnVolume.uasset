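; SpawnVolume is a spawn point that creates one randomized Musician at a time and holds it as an attached actor.
; Its SpawnMusician event waits briefly, then spawns only if nothing is attached to the volume.
; The new Musician gets a random job plus a sprite and texture sharing one random index.
; It spawns at the origin and attaches with keep-relative rules, placing it at the volume.
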(event `self.ReceiveBeginPlay`)

(event `SpawnMusician`
  (`KismetSystemLibrary.Delay` 1.0)
  (if (not (> (`KismetArrayLibrary.Array_Length` (`self.GetAttachedActors`)) 0))
    (set `self.Random` (`KismetMathLibrary.RandomInteger` 2))
    (bind _returnvalue (`|SpawnActorFromClass` "/Game/BluePrints/Musician.Musician_C" (`KismetMathLibrary.MakeTransform` (0.0 0.0 0.0) (struct)) "Undefined" "OverrideRootScale" null (`KismetArrayLibrary.Array_Get` (`self.Jobs`) (`KismetMathLibrary.RandomInteger` 4)) (`KismetArrayLibrary.Array_Get` (`self.Sprites`) (`self.Random`)) (`KismetArrayLibrary.Array_Get` (`self.Textures`) (`self.Random`)) (`self.Instigator`)))
    (`self.K2_AttachToActor` _returnvalue self "None" "KeepRelative" "KeepRelative" "KeepRelative" false)))

(fn `UserConstructionScript`)
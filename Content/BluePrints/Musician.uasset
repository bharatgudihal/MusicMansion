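; Musician actor: a tappable sprite character the player moves from the street into building rooms.
; A touch on the street hides it and shows its portrait and job via the GameMode; a touch while boxed checks the current room's job and free spot.
; Valid placement attaches it to the spot, updates counts and location state, and can start music writing in Recording rooms.
; Tick lerp-bounces it while a party is happening.
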(event `self.ReceiveTick`
  (params (DeltaSeconds :type "Float (single-precision)"))
  (`self.DoParty` 0.0))

(event `self.ReceiveBeginPlay`
  ;[1 1 1] Begin Play
  (set `self.locationState` "OnStreet")
  (bind _ascustom_game_mode (cast `/Game/BluePrints/CustomGameMode` (`GameplayStatics.GetGameMode`)))
  (set `self.GameMode` _ascustom_game_mode))

(event `self.ReceiveActorOnInputTouchEnd`
  (params (FingerIndex :type "ETouchIndex Enum" :default "Touch1"))
  ;[1 1 1] On Touch
  (`self.IsTouched`))

(fn `DisappearAndAppearInBox`
  (bind _gamemode (`self.GameMode`))
  (`ActorComponent.SetActive` (`self.StaticMeshComponent`) false false)
  (`SceneComponent.SetVisibility` (`self.PaperSprite`) false true)
  (set `/Game/BluePrints/CustomGameMode.PersonImage` (`self.Texture`) _gamemode)
  (set `/Game/BluePrints/CustomGameMode.PersonJob` (`KismetTextLibrary.Conv_StringToText` (`|GetEnumeratorNameAsString` (`self.Job`))) _gamemode))

(fn `DoParty`
  (params (DeltaTime :type "Float (double-precision)"))
  (if (`/Game/BluePrints/CustomGameMode.IsPartyHappening` (`self.GameMode`))
    (if (`self.Jump`)
      (bind _output_get (set `self.CurrentLocation` (`KismetMathLibrary.VLerp` (`self.CurrentLocation`) (0.0 0.0 10.0) 0.3)))
      (`self.K2_SetActorRelativeLocation` _output_get)
      (if (>= (.z (`self.CurrentLocation`)) 9.9)
        (set `self.Jump` false))
      (else
        (bind _output_get_2 (set `self.CurrentLocation` (`KismetMathLibrary.VLerp` (`self.CurrentLocation`) (0.0 0.0 0.0) 0.3)))
        (`self.K2_SetActorRelativeLocation` _output_get_2)
        (if (<= (.z (`self.CurrentLocation`)) 0.1)
          (set `self.Jump` true))))
    (else
      (`self.K2_SetActorRelativeLocation` (0.0 0.0 0.0)))))

(fn `FlashInvalidSelection`
  (`KismetSystemLibrary.PrintString` "They can't work there" true true (struct :`R` 1.0 :`B` 0.026227 :`A` 1.0)))

(fn `GetIsClicked`
  (returns (isClicked :type Boolean))
  (locals (justClicked :type Boolean))
  (bind (_bblockinghit _binitialoverlap _time _location _impactpoint _normal _impactnormal _physmat _hitactor _hitcomponent _hitbonename _hititem _faceindex _tracestart _traceend) (`GameplayStatics.BreakHitResult` (`PlayerController.GetHitResultUnderCursorByChannel` (`GameplayStatics.GetPlayerController` 0) "TraceTypeQuery2" true)))
  ;[1 1 1] GetIsClicked
  (bind _outhits (`KismetSystemLibrary.LineTraceMulti_NEW` :`Start` _tracestart :`End` _traceend :`TraceChannel` "TraceTypeQuery2" :`bIgnoreSelf` false))
  (for _array_element _outhits
    (bind _returnvalue (== (`.HitActor` (`GameplayStatics.BreakHitResult` _array_element)) self))
    (if (and true _returnvalue)
      (bind _output_get (set `local.justClicked` _returnvalue))
      (break)))
  (return _output_get))

(fn `IsTouched`
  (returns (Result :type Boolean))
  (bind _currentroom (`/Game/BluePrints/CustomGameMode.CurrentRoom` (`self.GameMode`)))
  (switch `string` (`self.locationState`)
    (:`OnStreet`
      (if true
        (`self.DisappearAndAppearInBox`)
        (if (!= null (`self.myApartment`))
          (`/Game/BluePrints/Room_BP.LeaveRoom` (`self.myApartment`) self))
        (set `self.locationState` "InBox")
        (return true)
        (else
          _)))
    (:`InBox`
      (if (!= (`self.myApartment`) null)
        (bind _hasavailable (`/Game/BluePrints/Room_BP.hasAvailableSpot` _currentroom))
        (if (and _hasavailable (`KismetArrayLibrary.Array_Contains` (`/Game/BluePrints/Room_BP.Jobs` _currentroom) (`self.Job`)))
          (bind _availablespot (`/Game/BluePrints/Room_BP.GetNextAvailableSpot` _currentroom self))
          (`self.SetNewParent` _availablespot)
          (switch `string` (`/Game/BluePrints/Room_BP.roomTypeName` (`/Game/BluePrints/CustomGameMode.CurrentRoom` (`self.GameMode`))) :!label _label
            (:`apartment`
              (set `self.locationState` "InApartment"))
            (:`recording`
              (set `self.locationState` "InRecording"))
            (:`party`
              (set `self.locationState` "InParty")))
          (return true)
          (else
            _))
        (else
          (bind _hasavailable_2 (`/Game/BluePrints/Room_BP.hasAvailableSpot` (`/Game/BluePrints/CustomGameMode.CurrentRoom` (`self.GameMode`))))
          (if _hasavailable_2
            (bind _isvalidapartment (`self.IsValidApartment`))
            (if _isvalidapartment
              (`self.SetApartment`)
              (bind _availablespot_2 (`/Game/BluePrints/Room_BP.GetNextAvailableSpot` (`self.myApartment`) self))
              (`self.SetNewParent` _availablespot_2)
              (goto _label)
              (else
                _)))))))
  (`self.FlashInvalidSelection`)
  (return false))

(fn `IsValidApartment`
  (returns (isValidApartment :type Boolean))
  (bind _gamemode (`self.GameMode`))
  (bind _currentroom (`/Game/BluePrints/CustomGameMode.CurrentRoom` _gamemode))
  (bind _returnvalue (and (not (`/Game/BluePrints/Room_BP.Working` _currentroom)) (not (`/Game/BluePrints/Room_BP.isRented` _currentroom)) (`KismetArrayLibrary.Array_Contains` (`/Game/BluePrints/Room_BP.Jobs` _currentroom) (`self.Job`)) (> (`/Game/BluePrints/CustomGameMode.BuildingCapacity` _gamemode) 0)))
  ;[1 1 1] Set Apartment
  (if _returnvalue
    _
    (else
      _))
  (return _returnvalue))

(fn `SetApartment`
  ;[1 1 1] SetApartment
  (set `self.myApartment` (`/Game/BluePrints/CustomGameMode.CurrentRoom` (`self.GameMode`))))

(fn `SetNewParent`
  (params (newParentActor :type "Actor Object Reference"))
  (bind _myapartment (`self.myApartment`))
  (`SceneComponent.SetVisibility` (`self.PaperSprite`) true true)
  (`self.K2_AttachToActor` newParentActor "None" "KeepRelative" "KeepRelative" "KeepWorld")
  (`self.K2_SetActorRotation` (struct :`Yaw` 90.0))
  (`/Game/BluePrints/CustomGameMode.SubPeople` (`self.GameMode`))
  ;[1 1 1] Notify Recording Room That Musician Is Writing
  (`/Game/BluePrints/Room_BP.AddPeep` _myapartment)
  (if (== _myapartment (`/Game/BluePrints/CustomGameMode.CurrentRoom` (`self.GameMode`)))
    (switch `string` (`/Game/BluePrints/Room_BP.roomTypeName` (`self.myApartment`))
      (:`recording`
        (set `self.isWritingMusic` true)
        (`/Game/BluePrints/Room_BP.SetIsMusicianWriting` (`self.myApartment`))))))

(fn `UserConstructionScript`
  (`PaperSpriteComponent.SetSprite` (`self.PaperSprite`) (`self.Sprite`)))
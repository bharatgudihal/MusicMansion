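; Building actor that assembles itself from floor and room actors, starting with floor 0 on BeginPlay.
; SpawnFloor spawns four Room_BP actors at the building's transform and passes them, with the floor number, into a new Floor_BP.
; Each new floor is attached to the building with keep-relative rules, added to the Floors array and counted in TotalFloorCount.
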(event `self.ReceiveBeginPlay`
  (`self.SpawnFloor` 0))

(fn `SpawnFloor`
  (params (FloorNumber :type Integer))
  (bind _returnvalue (`self.GetTransform`))
  (bind _instigator (`self.Instigator`))
  (bind _returnvalue_2 (`|SpawnActorFromClass` "/Game/BluePrints/Room_BP.Room_BP_C" _returnvalue "Undefined" "OverrideRootScale" null _instigator))
  (bind _returnvalue_3 (`|SpawnActorFromClass` "/Game/BluePrints/Room_BP.Room_BP_C" _returnvalue "Undefined" "OverrideRootScale" null _instigator))
  (bind _returnvalue_4 (`|SpawnActorFromClass` "/Game/BluePrints/Room_BP.Room_BP_C" _returnvalue "Undefined" "OverrideRootScale" null _instigator))
  (bind _returnvalue_5 (`|SpawnActorFromClass` "/Game/BluePrints/Room_BP.Room_BP_C" _returnvalue "Undefined" "OverrideRootScale" null _instigator))
  (bind _returnvalue_6 (`|SpawnActorFromClass` "/Game/BluePrints/Floor_BP.Floor_BP_C" _returnvalue "Undefined" "OverrideRootScale" null _returnvalue_2 _returnvalue_3 _returnvalue_4 _returnvalue_5 FloorNumber _instigator))
  (`self.K2_AttachToActor` _returnvalue_6 self "None" "KeepRelative" "KeepRelative" "KeepRelative" true)
  (`KismetArrayLibrary.Array_Add` (`self.Floors`) _returnvalue_6)
  (`/Engine/EditorBlueprintResources/StandardMacros.IncrementInt` (`self.TotalFloorCount`)))

(fn `UserConstructionScript`)
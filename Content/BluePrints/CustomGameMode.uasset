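; Game mode for a music-themed idle game that tracks money, songs, parties and the active room in a rotating multi-floor building.
; Swipe events queue 90-degree turns animated on Tick or move the player's target between floors, updating the active room.
; Tick also totals room income, banks capped earnings until the Collect button adds them, and hides spawn actors while a room is selected.
; A looping timer spawns musicians.
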(event `self.ReceiveBeginPlay`)

(event `Begin`
  (`self.SetCurrentRoom`)
  (bind _returnvalue (`|CreateWidget` "/Game/BluePrints/GeneralUI_BP.GeneralUI_BP_C" null (`self.Player`)))
  (bind _output_get (set `self.UI` _returnvalue))
  (`UserWidget.AddToViewport` _output_get 0)
  (add `Button.OnClicked` (`/Game/BluePrints/GeneralUI_BP.CollectButton` _output_get) (delegate `AddTempMoney`))
  (`KismetSystemLibrary.K2_SetTimerDelegate` (delegate `SpawnMusician`) 5.0 true))

(event `SpawnMusician`
  (`/Game/BluePrints/SpawnVolume.SpawnMusician` (`self.SpawnVolume`)))

(event `AddTempMoney`
  (`self.Addmoney`))

(event `self.ReceiveTick`
  (params (DeltaSeconds :type "Float (single-precision)"))
  (`self.RotateBuildingLeft` DeltaSeconds)
  (`self.RotateBuildingRight` DeltaSeconds)
  (`self.UpdateHUD`)
  (`self.ShowAuxillaryActors`))

(event `Left`
  ;[1 1 1] Set the rotation to which the building has to rotate to when swiped left
  (if (not (or (`self.rotateLeft`) (`self.rotateRight`) (`/Game/BluePrints/Room_BP.IsSelected` (`self.CurrentRoom`))))
    (bind _output_get (set `self.rotateTo` (`KismetMathLibrary.MakeRotator` (.roll (`self.K2_GetActorRotation` (`self.Building`))) (.pitch (`self.K2_GetActorRotation` (`self.Building`))) (+ (.yaw (`self.K2_GetActorRotation` (`self.Building`))) 90.0))))
    (bind _yaw (.yaw _output_get))
    (if (> _yaw 180.0)
      (set `self.rotateTo` (`KismetMathLibrary.MakeRotator` (.roll _output_get) (.pitch _output_get) (- _yaw 360.0)))
      (set `self.rotateLeft` true)
      (else
        (set `self.rotateLeft` true)))))

(event `Right`
  ;[1 1 1] Set the rotation to which the building has to rotate to when swiped right
  (if (not (or (`self.rotateLeft`) (`self.rotateRight`) (`/Game/BluePrints/Room_BP.IsSelected` (`self.CurrentRoom`))))
    (bind _output_get (set `self.rotateTo` (`KismetMathLibrary.MakeRotator` (.roll (`self.K2_GetActorRotation` (`self.Building`))) (.pitch (`self.K2_GetActorRotation` (`self.Building`))) (+ (.yaw (`self.K2_GetActorRotation` (`self.Building`))) -90.0))))
    (bind _yaw (.yaw _output_get))
    (if (< _yaw -180.0)
      (set `self.rotateTo` (`KismetMathLibrary.MakeRotator` (.roll _output_get) (.pitch _output_get) (+ _yaw 360.0)))
      (set `self.rotateRight` true)
      (else
        (set `self.rotateRight` true)))))

(event `Up`
  (bind _currentfloor (`self.CurrentFloor`))
  (if (and (< _currentfloor (`/Game/BluePrints/Building_BP.TotalFloorCount` (`self.Building`))) (not (`/Game/BluePrints/Room_BP.IsSelected` (`self.CurrentRoom`))))
    (`CameraElevator.SetTargetUp` (`self.Player`))
    (`/Engine/EditorBlueprintResources/StandardMacros.IncrementInt` _currentfloor
      (:`  `
        (`self.SetCurrentRoom`)))))

(event `Down`
  (bind _currentfloor (`self.CurrentFloor`))
  (if (and (> _currentfloor 1) (not (`/Game/BluePrints/Room_BP.IsSelected` (`self.CurrentRoom`))))
    (`CameraElevator.SetTargetDown` (`self.Player`))
    (`/Engine/EditorBlueprintResources/StandardMacros.DecrementInt` _currentfloor
      (:`  `
        (`self.SetCurrentRoom`)))))

(event `UpdateHUD`
  (`self.UpdateHUDValues`))

(fn `Addmoney`
  (set `self.TotalMoney` (+ (`self.TotalMoney`) (`self.TempTotalMoney`)))
  (set `self.TempTotalMoney` 0.0)
  (for _array_element (`/Game/BluePrints/Building_BP.Floors` (`self.Building`))
    (for _array_element_2 (`|MakeArray` (`/Game/BluePrints/Floor_BP.Room0` _array_element) (`/Game/BluePrints/Floor_BP.Room1` _array_element) (`/Game/BluePrints/Floor_BP.Room2` _array_element) (`/Game/BluePrints/Floor_BP.Room3` _array_element))
      (if (`/Game/BluePrints/Room_BP.IsScheduleForMoneyReset` _array_element_2)
        (set `/Game/BluePrints/Room_BP.IsScheduleForMoneyReset` false _array_element_2)
        (set `/Game/BluePrints/Room_BP.RoomMoney` 0.0 _array_element_2)))))

(fn `AddNewSong`
  (set `self.songsMade` (+ (`self.songsMade`) 1)))

(fn `DeductMoney`
  (params (Cost :type "Float (double-precision)"))
  (returns (State :type Boolean))
  (bind _totalmoney (`self.TotalMoney`))
  (if (<= Cost _totalmoney)
    (set `self.TotalMoney` (- _totalmoney Cost))
    (return true)
    (else
      (return false))))

(fn `GetCanThrowParty`
  (returns (canThrowParty :type Boolean))
  (locals (canThrow :type Boolean))
  (bind _output_get (set `local.canThrow` (> (`self.songsMade`) (`self.partiesThrown`))))
  (return _output_get))

(fn `RotateBuildingLeft`
  (params (DeltaTime :type "Float (double-precision)"))
  (bind _building (`self.Building`))
  (bind _currentroomnumber (`self.CurrentRoomNumber`))
  (bind _yaw (.yaw (`self.rotateTo`)))
  (bind _yaw_2 (.yaw (`self.K2_GetActorRotation` _building)))
  (if (`self.rotateLeft`)
    (`self.K2_AddActorLocalRotation` _building (`KismetMathLibrary.MakeRotator` 0.0 0.0 (* DeltaTime (`self.RotateSpeed`))) false false)
    (if (< _yaw 0.0)
      (bind _output_get (set `self.rotateLeft` (> (`KismetMathLibrary.Abs` _yaw_2) (`KismetMathLibrary.Abs` _yaw))))
      (if (not _output_get)
        (`self.K2_SetActorRotation` (`self.Building`) (`self.rotateTo`) false)
        (`/Engine/EditorBlueprintResources/StandardMacros.IncrementInt` _currentroomnumber :!label _label
          (:`  `
            (if (> _currentroomnumber 4)
              (set `self.CurrentRoomNumber` 1))
            (`self.SetCurrentRoom`))))
      (else
        (bind _output_get_2 (set `self.rotateLeft` (> _yaw _yaw_2)))
        (if (not _output_get_2)
          (`self.K2_SetActorRotation` (`self.Building`) (`self.rotateTo`) false)
          (goto _label))))))

(fn `RotateBuildingRight`
  (params (DeltaTime :type "Float (double-precision)"))
  (bind _building (`self.Building`))
  (bind _currentroomnumber (`self.CurrentRoomNumber`))
  (bind _yaw (.yaw (`self.rotateTo`)))
  (bind _yaw_2 (.yaw (`self.K2_GetActorRotation` _building)))
  ;[1 1 1] Rotate Right
  (if (`self.rotateRight`)
    (`self.K2_AddActorLocalRotation` _building (`KismetMathLibrary.MakeRotator` 0.0 0.0 (* DeltaTime (- 0.0 (`self.RotateSpeed`)))) true false)
    (if (> _yaw 0.0)
      (bind _output_get (set `self.rotateRight` (> (`KismetMathLibrary.Abs` _yaw_2) _yaw)))
      (if (not _output_get)
        (`self.K2_SetActorRotation` (`self.Building`) (`self.rotateTo`) false)
        (`/Engine/EditorBlueprintResources/StandardMacros.DecrementInt` _currentroomnumber :!label _label
          (:`  `
            (if (< _currentroomnumber 1)
              (set `self.CurrentRoomNumber` 4))
            (`self.SetCurrentRoom`))))
      (else
        (bind _output_get_2 (set `self.rotateRight` (> _yaw_2 _yaw)))
        (if (not _output_get_2)
          (`self.K2_SetActorRotation` (`self.Building`) (`self.rotateTo`) false)
          (goto _label))))))

(fn `SetCurrentRoom`
  (bind _currentroom (`self.CurrentRoom`))
  (bind _item (`KismetArrayLibrary.Array_Get` (`/Game/BluePrints/Building_BP.Floors` (`self.Building`)) (- (`self.CurrentFloor`) 1)))
  (bind _room0 (`/Game/BluePrints/Floor_BP.Room0` _item))
  (bind _room1 (`/Game/BluePrints/Floor_BP.Room1` _item))
  (bind _room2 (`/Game/BluePrints/Floor_BP.Room2` _item))
  (bind _room3 (`/Game/BluePrints/Floor_BP.Room3` _item))
  (`/Engine/EditorBlueprintResources/StandardMacros.IsValid` _currentroom
    (:`Is Valid`
      (set `/Game/BluePrints/Room_BP.IsActive` false _currentroom))
    (:`Is Not Valid`
      _))
  (switch `int` (`self.CurrentRoomNumber`)
    (:`1`
      (set `/Game/BluePrints/Room_BP.IsActive` true _room0)
      (set `self.CurrentRoom` _room0))
    (:`2`
      (set `/Game/BluePrints/Room_BP.IsActive` true _room1)
      (set `self.CurrentRoom` _room1))
    (:`3`
      (set `/Game/BluePrints/Room_BP.IsActive` true _room2)
      (set `self.CurrentRoom` _room2))
    (:`4`
      (set `/Game/BluePrints/Room_BP.IsActive` true _room3)
      (set `self.CurrentRoom` _room3))))

(fn `ShowAuxillaryActors`
  (bind _spawnvolume (`self.SpawnVolume`))
  (bind _isselected (`/Game/BluePrints/Room_BP.IsSelected` (`self.CurrentRoom`)))
  (bind _item (`KismetArrayLibrary.Array_Get` (`self.GetAttachedActors` _spawnvolume)))
  (`self.SetActorHiddenInGame` _spawnvolume _isselected)
  (`/Engine/EditorBlueprintResources/StandardMacros.IsValid` _item
    (:`Is Valid`
      (`self.SetActorHiddenInGame` _item _isselected))))

(fn `ThrowParty`
  (set `self.partiesThrown` (+ (`self.partiesThrown`) 1)))

(fn `UpdateHUDValues`
  (locals (PerSecondMoneyTotal :type "Float (double-precision)"))
  (for _array_element (`/Game/BluePrints/Building_BP.Floors` (`self.Building`))
    (bind _room0 (`/Game/BluePrints/Floor_BP.Room0` _array_element))
    (bind _room1 (`/Game/BluePrints/Floor_BP.Room1` _array_element))
    (bind _room2 (`/Game/BluePrints/Floor_BP.Room2` _array_element))
    (bind _room3 (`/Game/BluePrints/Floor_BP.Room3` _array_element))
    (set `local.PerSecondMoneyTotal` (+ (`/Game/BluePrints/Room_BP.MoneyPerFrame` _room0) (`/Game/BluePrints/Room_BP.MoneyPerFrame` _room1) (`/Game/BluePrints/Room_BP.MoneyPerFrame` _room2) (`/Game/BluePrints/Room_BP.MoneyPerFrame` _room3) (`local.PerSecondMoneyTotal`)))
    (for _array_element_2 (`|MakeArray` _room0 _room1 _room2 _room3)
      (if (`/Game/BluePrints/Room_BP.IsMoneyCapReached` _array_element_2)
        (set `/Game/BluePrints/Room_BP.IsMoneyCapReached` false _array_element_2)
        (set `self.TempTotalMoney` (+ (`/Game/BluePrints/Room_BP.RoomMoneyCap` _array_element_2) (`self.TempTotalMoney`)))
        (set `/Game/BluePrints/Room_BP.IsScheduleForMoneyReset` true _array_element_2))))
  (set `self.MoneyPerSecond` (* (`local.PerSecondMoneyTotal`) 60.0)))

(fn `UserConstructionScript`)
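; Buildable room actor that becomes an apartment, recording studio or party room and accrues capped income.
; Its UI buttons charge CustomGameMode and start construction, with a progress widget shown until completion.
; Tick drives the selection slide lerp, frame-counted build progress and per-frame income, so timing depends on frame rate.
; BeginPlay spawns person anchors at nine floor spots for free-spot lookup; touch selection is blocked by a hard-coded false condition.
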(event `self.ReceiveBeginPlay`
  ;[1 1 1] Initialize_RoomBP
  ;;[1 1 1] AttachUIElements
  (set `self.MoveTo` (`self.K2_GetActorLocation`))
  (bind _returnvalue (`|CreateWidget` "/Game/BluePrints/BuildRoomUI.BuildRoomUI_C"))
  (bind _output_get (set `self.BuildRoomUI` _returnvalue))
  (add `Button.OnClicked` (`/Game/BluePrints/BuildRoomUI.RoomAButton` _output_get) (delegate `ClickApartmentRoom`))
  ;;[1 1 1] Bind BuildRoom - Recording
  (add `Button.OnClicked` (`/Game/BluePrints/BuildRoomUI.RoomBButton` _output_get) (delegate `ClickRecordingStudio`))
  (add `Button.OnClicked` (`/Game/BluePrints/BuildRoomUI.RoomCButton` _output_get) (delegate `ClickPartyRoom`))
  (bind _ascustom_game_mode (cast `/Game/BluePrints/CustomGameMode` (`GameplayStatics.GetGameMode`)))
  (set `self.GameMode` _ascustom_game_mode)
  ;[1 1 1] InitializeChildActors
  (set `self.allFloorSpots` (`|MakeArray` (`self.StaticMesh`) (`self.StaticMesh1`) (`self.StaticMesh2`) (`self.StaticMesh3`) (`self.StaticMesh4`) (`self.StaticMesh5`) (`self.StaticMesh6`) (`self.StaticMesh7`) (`self.StaticMesh8`)))
  (for _array_element (`self.allFloorSpots`)
    (bind _returnvalue_2 (`|SpawnActorFromClass` "/Game/BluePrints/personAnchorActor_Blueprint.personAnchorActor_Blueprint_C" (`self.GetTransform`) "AlwaysSpawn" "OverrideRootScale" null (`self.Instigator`)))
    (`KismetArrayLibrary.Array_Add` (`self.allFloorAnchors`) _returnvalue_2)
    (`self.K2_AttachToActor` _returnvalue_2 self "None" "KeepRelative" "KeepRelative" "KeepRelative" true)
    (`self.K2_SetActorLocation` _returnvalue_2 (`SceneComponent.K2_GetComponentLocation` _array_element) false false)))

(event `self.ReceiveTick`
  (params (DeltaSeconds :type "Float (single-precision)"))
  ;[1 1 1] Tick
  (`self.LerpRoomToSelectionPosition`)
  (`self.CalculateBuildPercentage`)
  (`self.AddMoney`))

(event `self.ReceiveActorOnInputTouchEnd`
  (params (FingerIndex :type "ETouchIndex Enum" :default "Touch1"))
  (bind _gamemode (`self.GameMode`))
  (bind (_bblockinghit _binitialoverlap _time _location _impactpoint _normal _impactnormal _physmat _hitactor) (`GameplayStatics.BreakHitResult` (`PlayerController.GetHitResultUnderCursorByChannel` (`GameplayStatics.GetPlayerController` 0) "TraceTypeQuery2" true)))
  ;[1 1 1] OnTouch
  (if (and (`self.IsActive`) (not (`self.Working`)) false (not (`/Game/BluePrints/CustomGameMode.rotateLeft` _gamemode)) (not (`/Game/BluePrints/CustomGameMode.rotateRight` _gamemode)) (not (`self.IsSelectionAnimationPlaying`)))
    (if (== _hitactor self)
      (`self.ToggleIsSelected`)
      (else
        (bind _asmusician (cast `/Game/BluePrints/Musician` _hitactor))
        (`/Game/BluePrints/Musician.InvokeTouch` _asmusician)))))

(event `ClickApartmentRoom`
  ;[1 1 1] Initialize_RoomBP
  ;;[1 1 1] Bind BuildRoom - Apartment
  (bind _state (`/Game/BluePrints/CustomGameMode.DeductMoney` (`self.GameMode`) 100.0))
  (if _state
    (`PrimitiveComponent.SetMaterial` (`self.StaticMeshComponent`) 0 "/Game/Assets/lambert3.lambert3")
    (`self.ToggleIsSelected`)
    (set `self.RoomType` 1)
    (set `self.NumberOfFramesToComplete` 100.0)
    (set `self.Cost` 100.0)
    ;;[1 1 1] CompleteRoomConstruction
    (`Widget.SetVisibility` (`WidgetComponent.GetUserWidgetObject` (`self.Widget`)) "Visible" :!label _label)
    (set `self.Working` true)
    (set `self.PercentageComplete` 0.0)
    (set `self.IsBuilt` false)
    (bind _ascustom_game_mode (cast `/Game/BluePrints/CustomGameMode` (`GameplayStatics.GetGameMode`)))
    (`/Game/BluePrints/CustomGameMode.RoomTapped` _ascustom_game_mode (`self.Cost`))
    (switch `int` (`self.RoomType`)
      (:`1`
        (set `self.roomTypeName` "apartment"))
      (:`2`
        (set `self.roomTypeName` "recording"))
      (:`3`
        (set `self.roomTypeName` "party")))))

(event `ClickRecordingStudio`
  ;[1 1 1] Initialize_RoomBP
  ;;[1 1 1] Bind BuildRoom - Recording
  (bind _state (`/Game/BluePrints/CustomGameMode.DeductMoney` (`self.GameMode`) 200.0))
  (if _state
    (`PrimitiveComponent.SetMaterial` (`self.StaticMeshComponent`) 0 "/Game/Assets/lambert4.lambert4")
    (`self.ToggleIsSelected`)
    (set `self.RoomType` 2)
    (set `self.NumberOfFramesToComplete` 100.0)
    (set `self.Cost` 200.0)
    (goto _label)))

(event `ClickPartyRoom`
  ;[1 1 1] Initialize_RoomBP
  ;;[1 1 1] BindBuildRoom - Party
  (bind _state (`/Game/BluePrints/CustomGameMode.DeductMoney` (`self.GameMode`) 300.0))
  (if _state
    (`PrimitiveComponent.SetMaterial` (`self.StaticMeshComponent`) 0 "/Game/Assets/lambert5.lambert5")
    (`self.ToggleIsSelected`)
    (set `self.RoomType` 3)
    (set `self.NumberOfFramesToComplete` 100.0)
    (set `self.Cost` 300.0)
    (goto _label)))

(fn `AddMoney`
  (bind _roommoneycap (`self.RoomMoneyCap`))
  (if (and (not (`self.IsScheduleForMoneyReset`)) (not (`self.Working`)))
    (bind _output_get (set `self.RoomMoney` (+ (`self.RoomMoney`) (`self.MoneyPerFrame`))))
    (if (< _roommoneycap _output_get)
      (set `self.RoomMoney` _roommoneycap)
      (set `self.IsMoneyCapReached` true))))

(fn `AddRenter`
  (set `self.isRented` true))

(fn `CalculateBuildPercentage`
  (if (and (`self.Working`) (not (`self.IsBuilt`)))
    (if (== (`self.PercentageComplete`) 1.0)
      (set `self.FrameNumber` 0.0)
      (set `self.NumberOfFramesToComplete` 0.0)
      (`Widget.SetVisibility` (`WidgetComponent.GetUserWidgetObject` (`self.Widget`)) "Hidden")
      (set `self.Working` false)
      (set `self.IsBuilt` true)
      (switch `int` (`self.RoomType`)
        (:`1`
          (set `self.NumberOfFramesToComplete` 3600.0)
          (set `self.MoneyPerFrame` 0.008)
          (set `self.RoomMoneyCap` 200.0))
        (:`2`
          (set `self.NumberOfFramesToComplete` 3600.0)
          (set `self.MoneyPerFrame` 0.016)
          (set `self.RoomMoneyCap` 600.0))
        (:`3`
          (set `self.NumberOfFramesToComplete` 3600.0)
          (set `self.MoneyPerFrame` 0.032)
          (set `self.RoomMoneyCap` 1000.0)))
      (else
        (bind _result (`/Engine/EditorBlueprintResources/StandardMacros.IncrementFloat` (`self.FrameNumber`))
          (:`  `
            (set `self.PercentageComplete` (/ _result (`self.NumberOfFramesToComplete`)))))))))

(fn `GetNextAvailableSpot`
  (returns (availableSpot :type "Actor Object Reference"))
  ;[1 1 1] GetNextAvailableSpot
  (for _array_element (`self.allFloorAnchors`)
    (if (== (`KismetArrayLibrary.Array_Length` (`self.GetAttachedActors` _array_element)) 0)
      (break)))
  (return _array_element))

(fn `HasAvailableSpot`
  (returns (hasAvailable :type Boolean))
  ;[1 1 1] HasAvailableSpot
  (for _array_element (`self.allFloorAnchors`)
    (if (== (`KismetArrayLibrary.Array_Length` (`self.GetAllChildActors` _array_element false)) 0)
      (break)))
  (return (`self.hasAvailable`)))

(fn `LerpRoomToSelectionPosition`
  (bind _moveto (`self.MoveTo`))
  (if (`self.IsSelectionAnimationPlaying`)
    (`self.K2_SetActorLocation` (`KismetMathLibrary.VLerp` (`self.K2_GetActorLocation`) (`self.MoveTo`) 0.2))
    (if (== (`self.K2_GetActorLocation`) _moveto :`ErrorTolerance` 0.1)
      (set `self.IsSelectionAnimationPlaying` false)
      (`self.K2_SetActorLocation` _moveto))))

(fn `ToggleIsSelected`
  (bind _returnvalue (`self.K2_GetActorLocation`))
  ;[1 1 1] ToggleIsSelected
  (if (`self.IsSelected`)
    (set `self.MoveTo` (+ _returnvalue (25.0 0.0 -25.0)))
    (set `self.IsSelected` false)
    (else
      (set `self.MoveTo` (+ _returnvalue (-25.0 0.0 25.0)))
      (set `self.IsSelected` true)))
  (set `self.IsSelectionAnimationPlaying` true)
  (if (`self.IsSelected`)
    (`UserWidget.AddToViewport` (`self.BuildRoomUI`) 0)
    (else
      (`Widget.RemoveFromParent` (`self.BuildRoomUI`)))))

(fn `UserConstructionScript`
  (bind _returnvalue (`WidgetComponent.GetUserWidgetObject` (`self.Widget`)))
  (bind _asbuilding_room_ui (cast `/Game/BluePrints/BuildingRoomUI` _returnvalue))
  (set `/Game/BluePrints/BuildingRoomUI.Room` self _asbuilding_room_ui)
  (`Widget.SetVisibility` _returnvalue "Hidden"))
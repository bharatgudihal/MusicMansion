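; Person is an actor the player drags around the screen by touching its static mesh.
; Touch begin and end toggle a moving flag; while set, Tick maps the first touch's screen position to a world location relative to the camera elevator, at the horizontal distance measured on BeginPlay.
; Screen-to-world scale factors are precomputed once from the camera's field of view and aspect ratio, tuned with hard-coded constants.
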(event `self.StaticMeshComponent.OnInputTouchBegin`
  (params (FingerIndex :type "ETouchIndex Enum" :default "Touch1") (TouchedComponent :type "PrimitiveComponent Object Reference"))
  (set `self.isMoving` true))

(event `self.StaticMeshComponent.OnInputTouchEnd`
  (params (FingerIndex :type "ETouchIndex Enum" :default "Touch1") (TouchedComponent :type "PrimitiveComponent Object Reference"))
  (set `self.isMoving` false))

(event `self.ReceiveBeginPlay`
  (set `self.distanceAwayFromCamera` (`self.GetHorizontalDistanceTo` (`self.myCameraElevator`)))
  (`self.SetCameraToWorldSpaceMultipliers`))

(event `self.ReceiveTick`
  (params (DeltaSeconds :type "Float (single-precision)"))
  (if (`self.isMoving`)
    (`self.MoveWithTouch`)))

(fn `MoveWithTouch`
  (bind _returnvalue (`GameplayStatics.GetPlayerController` 0))
  (bind (_sizex _sizey) (`PlayerController.GetViewportSize` _returnvalue))
  (bind (_locationx _locationy) (`PlayerController.GetInputTouchState` _returnvalue "Touch1"))
  (if (`self.isMoving`)
    (`self.K2_SetActorLocation` (`KismetMathLibrary.MakeVector` (+ (`self.distanceAwayFromCamera`) (.x (`self.K2_GetActorLocation` (`self.myCameraElevator`)))) (+ (.y (`self.K2_GetActorLocation` (`self.myCameraElevator`))) (* (+ _locationx (* (`KismetMathLibrary.Conv_IntToDouble` _sizex) -0.5)) (`self.cameraToWorldSpaceMultiplierX`))) (+ (.z (`self.K2_GetActorLocation` (`self.myCameraElevator`))) (* (`self.cameraToWorldSpaceMultiplierY`) (+ _locationy (* (`KismetMathLibrary.Conv_IntToDouble` _sizey) -0.21))))))))

(fn `SetCameraToWorldSpaceMultipliers`
  (bind _camera (`/Game/BluePrints/MyCameraElevator_BP.Camera` (`self.myCameraElevator`)))
  (bind _output_get (set `self.realPlaneWidth` (* (* (`self.distanceAwayFromCamera`) 2.0) (`KismetMathLibrary.DegTan` (* 0.5 (`CameraComponent.FieldOfView` _camera))))))
  (set `self.cameraToWorldSpaceMultiplierX` (* 0.000775 _output_get))
  (bind _output_get_2 (set `self.realPlaneHeight` (* _output_get (`CameraComponent.AspectRatio` _camera))))
  (set `self.cameraToWorldSpaceMultiplierY` (* -0.0016 _output_get_2)))

(fn `UserConstructionScript`)
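; Dropbox_ForPeople is a Blueprint drop slot for people that shows the job of whoever is attached to it.
; Each tick it checks its attached actors and casts the first to Musician, writing that Musician's Job enum to a TextRender.
; With nothing attached it shows DefaultText, and if the cast fails the text stays unchanged.
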(event `self.ReceiveBeginPlay`)

(event `self.ReceiveTick`
  (params (DeltaSeconds :type "Float (single-precision)"))
  (bind _outactors (`self.GetAttachedActors`))
  (bind _textrender (`self.TextRender`))
  (if (> (`KismetArrayLibrary.Array_Length` _outactors) 0)
    (bind _asmusician (cast `/Game/BluePrints/Musician` (`KismetArrayLibrary.Array_Get` _outactors)))
    (`TextRenderComponent.K2_SetText` _textrender (`KismetTextLibrary.Conv_StringToText` (`|GetEnumeratorNameAsString` (`/Game/BluePrints/Musician.Job` _asmusician))))
    (else
      (`TextRenderComponent.K2_SetText` _textrender (`self.DefaultText`)))))

(fn `UserConstructionScript`)